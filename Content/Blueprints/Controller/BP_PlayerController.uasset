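; Player controller that relays player input to the controlled BP_ParentPawn and handles exiting the game mode.
; Movement axes call MoveLeft and MoveForward on the pawn, while hard-bound A or Q and D keys trigger LeftPressed and RightPressed.
; The Exit action calls Exit on GM_Standard, and each handler casts its target first, so input is ignored for other pawn or game mode types.
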(event `InputAxis|Move_Left`
  (params (AxisValue :type "Float (single-precision)"))
  (bind _asbp_parent_pawn (cast `/Game/Blueprints/Character/BP_ParentPawn` (`self.K2_GetPawn`)))
  (`/Game/Blueprints/Character/BP_ParentPawn.Move_Left` _asbp_parent_pawn AxisValue))

(event `InputAxis|Move_Forward`
  (params (AxisValue :type "Float (single-precision)"))
  (bind _asbp_parent_pawn (cast `/Game/Blueprints/Character/BP_ParentPawn` (`self.K2_GetPawn`)))
  (`/Game/Blueprints/Character/BP_ScrewPawn.Move_Forward` _asbp_parent_pawn AxisValue))

(event `Key|A`
  (params (Key :type "Key Structure"))
  (:`Pressed`
    (bind _asbp_parent_pawn (cast `/Game/Blueprints/Character/BP_ParentPawn` (`self.K2_GetPawn`) :!label _label))
    (`/Game/Blueprints/Character/BP_ParentPawn.Left_Pressed` _asbp_parent_pawn)))

(event `Key|Q`
  (params (Key :type "Key Structure"))
  (:`Pressed`
    (goto _label)))

(event `Key|D`
  (params (Key :type "Key Structure"))
  (:`Pressed`
    (bind _asbp_parent_pawn (cast `/Game/Blueprints/Character/BP_ParentPawn` (`self.K2_GetPawn`)))
    (`/Game/Blueprints/Character/BP_ParentPawn.RightPressed` _asbp_parent_pawn)))

(event `InputAction|Exit`
  (params (Key :type "Key Structure"))
  (:`Pressed`
    (bind _asgm_standard (cast `/Game/Blueprints/Gamemode/GM_Standard` (`GameplayStatics.GetGameMode`)))
    (`/Game/Blueprints/Gamemode/GM_Standard.Exit` _asgm_standard)))

(fn `UserConstructionScript`)