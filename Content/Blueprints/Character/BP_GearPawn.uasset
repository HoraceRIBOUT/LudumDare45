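; Pawn driven by alternating left/right presses instead of standard forward input, which it overrides to do nothing.
; The interval between alternate presses, growing each Tick, sets how far Pivot rolls toward 90 degrees either side, so quick alternation keeps it upright.
; A press after a near-full interval flips the lean side.
; Until almost flat, Tick moves it along CameraPivot's forward vector and yaws that pivot with the roll.
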(event `self.ReceiveBeginPlay`)

(event `Print`
  (`KismetSystemLibrary.PrintString` "Hello"))

(event `/Game/Blueprints/Character/BP_ParentPawn.Move_Forward`
  (params (Value :type "Float (single-precision)"))
  ;[1 1 1] Override parent function (This pawn cannot move with ZQSD keys)
)

(event `/Game/Blueprints/Character/BP_ParentPawn.Left_Pressed`
  (bind _returnvalue (`KismetSystemLibrary.GetGameTimeInSeconds`))
  (if (not (`self.LeftIsLast`))
    (set `self.LeftIsLast` true)
    (bind _output_get (set `self.TimeBetweenInputs` (- _returnvalue (`self.LastInputTime`)) :!label _label))
    (set `self.LastInputTime` _returnvalue)
    (if (`self.LeftSide`)
      (bind _returnvalue_2 (`KismetMathLibrary.FClamp` (/ _output_get (`self.Rate`))))
      (bind _returnvalue_3 (>= _returnvalue_2 0.99))
      (set `self.LeftSide` (select `bool` _returnvalue_3 :`false` true))
      (`SceneComponent.K2_SetRelativeRotation` (`self.Pivot`) (`KismetMathLibrary.RLerp` (struct) (`KismetMathLibrary.MakeRotator` 90.0) _returnvalue_2) false false :!label _label_2)
      (else
        (set `self.LeftSide` (select `bool` _returnvalue_3 :`true` true))
        (`SceneComponent.K2_SetRelativeRotation` (`self.Pivot`) (`KismetMathLibrary.RLerp` (struct) (`KismetMathLibrary.MakeRotator` -90.0) _returnvalue_2) false false :!label _label_3)))))

(event `/Game/Blueprints/Character/BP_ParentPawn.RightPressed`
  (if (`self.LeftIsLast`)
    (set `self.LeftIsLast` false)
    (goto _label)))

(event `self.ReceiveTick`
  (params (DeltaSeconds :type "Float (single-precision)"))
  (bind _relativerotation_roll (`KismetMathLibrary.BreakRotator` (`SceneComponent.RelativeRotation` (`self.Pivot`))))
  (bind _returnvalue (`KismetMathLibrary.Abs` _relativerotation_roll))
  (if (<= _returnvalue 89.0)
    (`self.AddMovementInput` (`SceneComponent.GetForwardVector` (`self.CameraPivot`)) (* DeltaSeconds 15.0))
    (`SceneComponent.K2_SetRelativeRotation` (`self.CameraPivot`) (`KismetMathLibrary.RLerp` (struct) (`KismetMathLibrary.MakeRotator` 0.0 0.0 _relativerotation_roll) (/ _returnvalue 45.0)) false false))
  (set `self.TimeBetweenInputs` (+ (`self.TimeBetweenInputs`) DeltaSeconds))
  (if (`self.LeftSide`)
    (goto _label_2)
    (else
      (goto _label_3))))

(fn `UserConstructionScript`
  (`parent.UserConstructionScript`))