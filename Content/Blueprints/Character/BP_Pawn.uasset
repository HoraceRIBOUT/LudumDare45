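; BP_Pawn is a movable pawn whose camera pivot sways from side to side as it moves.
; Non-zero Move_Forward input yaws CameraPivot and Pivot together, scaled by frame time, with the CamRight flag flipping direction at fixed yaw limits.
; The same input drives movement along CameraPivot's forward vector, so the heading follows the sway.
; Mouse X yaws the collision component to turn the pawn.
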(event `InputAxis|Move_Forward`
  (params (AxisValue :type "Float (single-precision)"))
  (bind _camerapivot (`self.CameraPivot`))
  (bind _camerapivot_2 (`self.CameraPivot`))
  (bind _returnvalue (* AxisValue (`GameplayStatics.GetWorldDeltaSeconds`) 10.0))
  (bind (_relativerotation_roll _relativerotation_pitch _relativerotation_yaw) (`KismetMathLibrary.BreakRotator` (`SceneComponent.RelativeRotation` _camerapivot_2)))
  (bind (_relativerotation_roll_2 _relativerotation_pitch_2 _relativerotation_yaw_2) (`KismetMathLibrary.BreakRotator` (`SceneComponent.RelativeRotation` _camerapivot)))
  (`|ExecutionSequence`
    (:`then_0`
      (if (!= AxisValue 0.0)
        (if (`self.camRight`)
          (`SceneComponent.K2_AddRelativeRotation` _camerapivot (`KismetMathLibrary.MakeRotator` 0.0 0.0 (* _returnvalue -1.0)) false false)
          (`SceneComponent.K2_AddRelativeRotation` (`self.Pivot`) (`KismetMathLibrary.MakeRotator` 0.0 0.0 (* _returnvalue -1.0)) false false)
          (if (<= _relativerotation_yaw_2 -20.0)
            (set `self.camRight` false))
          (else
            (`SceneComponent.K2_AddRelativeRotation` _camerapivot_2 (`KismetMathLibrary.MakeRotator` 0.0 0.0 _returnvalue) false false)
            (`SceneComponent.K2_AddRelativeRotation` (`self.Pivot`) (`KismetMathLibrary.MakeRotator` 0.0 0.0 _returnvalue) false false)
            (if (>= _relativerotation_yaw 20.0)
              (set `self.camRight` true))))))
    (:`then_1`
      (`self.AddMovementInput` (`SceneComponent.GetForwardVector` (`self.CameraPivot`)) AxisValue))))

(event `InputAxisKey|MouseX`
  (params (AxisValue :type "Float (single-precision)"))
  (`SceneComponent.K2_AddWorldRotation` (`self.CollisionComponent`) (`KismetMathLibrary.MakeRotator` 0.0 0.0 AxisValue) false false))

(fn `UserConstructionScript`)