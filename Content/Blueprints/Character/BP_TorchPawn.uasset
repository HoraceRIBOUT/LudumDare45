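; BP_TorchPawn is a character Blueprint with basic movement input and an upward thrust while Space is held.
; Space opens and closes a Gate on Tick, which adds a velocity-change impulse along CameraPivot's up vector until vertical speed exceeds a cap.
; Forward and sideways axes feed movement input along the actor's vectors, with the sideways value printed for debugging.
; A direct velocity-setting node is left unconnected.
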(event `self.ReceiveTick`
  (params (DeltaSeconds :type "Float (single-precision)"))
  (bind (_velocity_x _velocity_y _velocity_z) (`KismetMathLibrary.BreakVector` (`MovementComponent.Velocity` (`self.CharacterMovement`))))
  (`/Engine/EditorBlueprintResources/StandardMacros.Gate` true :!label _label
    (:`Exit`
      (if (<= _velocity_z 1000.0)
        (`CharacterMovementComponent.AddImpulse` (`self.CharacterMovement`) (* (`SceneComponent.GetUpVector` (`self.CameraPivot`)) 100.0) true)))))

(event `Key|SpaceBar`
  (params (Key :type "Key Structure"))
  (:`Pressed`
    (goto _label :!via `Open`))
  (:`Released`
    (goto _label :!via `Close`)))

(event `/Game/Blueprints/Character/BP_ParentPawn.Move_Forward`
  (params (Value :type "Float (single-precision)"))
  (`self.AddMovementInput` (`self.GetActorForwardVector`) (* Value 1000.0)))

(event `InputAxis|Move_Left`
  (params (AxisValue :type "Float (single-precision)"))
  (`KismetSystemLibrary.PrintString` (`KismetStringLibrary.Conv_DoubleToString` AxisValue))
  (`self.AddMovementInput` (`self.GetActorRightVector`) (* AxisValue 100.0)))

(fn `UserConstructionScript`
  (`parent.UserConstructionScript`))