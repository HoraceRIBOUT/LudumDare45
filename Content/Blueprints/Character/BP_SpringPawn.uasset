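; BP_SpringPawn is a spring-like pawn that moves only by hopping, with the parent's directional movement events overridden to do nothing.
; Space, when grounded, triggers Jump plus a forward impulse and plays a timeline that animates StaticMesh3's Z scale.
; Mouse X yaws the capsule to aim the hop.
; JumpingFrame is set on jump and cleared on Tick while grounded.
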(event `/Game/Blueprints/Character/BP_ParentPawn.RightPressed`
  ;[1 1 1] Override parent function (This pawn cannot move with ZQSD keys)
)

(event `/Game/Blueprints/Character/BP_ParentPawn.Move_Forward`
  (params (Value :type "Float (single-precision)"))
  ;[1 1 1] Override parent function (This pawn cannot move with ZQSD keys)
)

(event `/Game/Blueprints/Character/BP_ParentPawn.Left_Pressed`
  ;[1 1 1] Override parent function (This pawn cannot move with ZQSD keys)
)

(event `self.ReceiveTick`
  (params (DeltaSeconds :type "Float (single-precision)"))
  (if (`NavMovementComponent.IsMovingOnGround` (`self.CharacterMovement`))
    (set `self.JumpingFrame` false)))

(event `Key|SpaceBar`
  (params (Key :type "Key Structure"))
  (:`Pressed`
    (if (`NavMovementComponent.IsMovingOnGround` (`self.CharacterMovement`))
      (set `self.JumpingFrame` true)
      (`self.Jump`)
      (`CharacterMovementComponent.AddImpulse` (`self.CharacterMovement`) (* (`SceneComponent.GetForwardVector` (`self.CapsuleComponent`)) 40000.0) false)
      (bind (_direction _scaleforce) (`Timeline|Timeline_0` :!via `PlayFromStart`)
        (:`Update`
          (`SceneComponent.SetRelativeScale3D` (`self.StaticMesh3`) (`KismetMathLibrary.MakeVector` 1.0 1.0 _scaleforce)))))))

(event `InputAxisKey|MouseX`
  (params (AxisValue :type "Float (single-precision)"))
  (`SceneComponent.K2_AddWorldRotation` (`self.CapsuleComponent`) (`KismetMathLibrary.MakeRotator` 0.0 0.0 AxisValue) false false))

(fn `UserConstructionScript`
  (`parent.UserConstructionScript`))