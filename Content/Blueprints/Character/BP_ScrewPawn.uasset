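; BP_ScrewPawn is a pawn driven by a forward axis, with Wwise gear movement audio posted on BeginPlay.
; Non-zero input yaws Pivot and CameraPivot together, scaled by input and frame time.
; The CamRight flag flips the yaw direction at fixed left and right limits, creating a side-to-side sway during forward input.
; Movement input follows the CameraPivot forward vector, so the path weaves with the sway.
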(event `self.ReceiveBeginPlay`
  (`AkGameplayStatics.PostEvent` "/Game/SOUND/Events/Screw_Movement_Gears.Screw_Movement_Gears" self))

(event `self.Move_Forward`
  (params (Value :type "Float (single-precision)"))
  (bind _pivot (`self.Pivot`))
  (bind _returnvalue (* Value (`GameplayStatics.GetWorldDeltaSeconds`) 20.0))
  (bind (_relativerotation_roll _relativerotation_pitch _relativerotation_yaw) (`KismetMathLibrary.BreakRotator` (`SceneComponent.RelativeRotation` (`self.CameraPivot`))))
  (bind (_relativerotation_roll_2 _relativerotation_pitch_2 _relativerotation_yaw_2) (`KismetMathLibrary.BreakRotator` (`SceneComponent.RelativeRotation` (`self.CameraPivot`))))
  (`|ExecutionSequence`
    (:`then_0`
      (if (!= Value 0.0)
        (if (`self.camRight`)
          (`SceneComponent.K2_AddRelativeRotation` _pivot (`KismetMathLibrary.MakeRotator` 0.0 0.0 (* _returnvalue -1.0)) false false)
          (`SceneComponent.K2_AddRelativeRotation` (`self.CameraPivot`) (`KismetMathLibrary.MakeRotator` 0.0 0.0 (* _returnvalue -1.0)) false false)
          (if (<= _relativerotation_yaw_2 -20.0)
            (set `self.camRight` false))
          (else
            (`SceneComponent.K2_AddRelativeRotation` _pivot (`KismetMathLibrary.MakeRotator` 0.0 0.0 _returnvalue) false false)
            (`SceneComponent.K2_AddRelativeRotation` (`self.CameraPivot`) (`KismetMathLibrary.MakeRotator` 0.0 0.0 _returnvalue) false false)
            (if (>= _relativerotation_yaw 20.0)
              (set `self.camRight` true))))))
    (:`then_1`
      (`self.AddMovementInput` (`SceneComponent.GetForwardVector` (`self.CameraPivot`)) Value))))

(fn `UserConstructionScript`)